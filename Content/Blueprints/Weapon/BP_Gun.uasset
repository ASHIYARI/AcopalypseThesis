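; First-person player gun that supplies the audio, visual and HUD feedback for multi-ammo firing and reloading.
; Fire events pick muzzle flash, arm montage, gun animation and sound by ammo type, then play impact sounds and occasional player voice lines on living enemy or drone hits.
; Reload and empty-mag states drive HUD widgets, while secondary ammo types get ready cues.
; Tick smoothly aims the flashlight at the hit-trace point.
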(event EventReloadTriggerEvent
  ;[1 1 1] Play Reload Animation
  (Animation|Montage|PlayMontage (Variables|/Script/Acopalyps.AcopalypsCharacter|GetMesh1P (.AsBP%20First%20Person%20Character (Utilities|Casting|CastToBP_FirstPersonCharacter (Game|GetPlayerCharacter 0)))) "/Game/Animations/CharacterAnimation/PlayerCharacter/Reload_Montage.Reload_Montage"
    (:then
      (Components|Animation|PlayAnimation (Variables|Default|GetSkeletalMesh) "/Game/Animations/CharacterAnimation/PlayerCharacter/Pistol_Reload_Anim.Pistol_Reload_Anim" false)
      ;[1 1 1] HUD Reload
      (bind _returnvalue (UserInterface|CreateWidget "/Game/UserInterface/W_Reloading.W_Reloading_C"))
      (UserInterface|Viewport|AddtoViewport _returnvalue 0))))

(event EventReloadCompletedEvent
  ;[1 1 1] Event Reload Complete
  (Utilities|FlowControl|Sequence
    (:then_0
      (if (Variables|Default|GetbNoAmmo)
        (Widget|RemovefromParent (stale EventFireTriggerEvent _returnvalue))
        (Variables|Default|SetbNoAmmo false)))
    (:then_1
      (Widget|RemovefromParent (stale EventReloadTriggerEvent _returnvalue)))))

(event EventEmptyMagFireAttemptEvent
  ;[1 1 1] Skjutljud + Switch Ammo
  (Audio|SpawnSound2D "/Game/Audio/SFX/Player/Weapon/Management/Switch/EmptyMagCue.EmptyMagCue" 1.0 1.0 0.0 0))

(event EventFireTriggerEvent
  (params (Hit :type Hit%20Result%20Structure%20%28by%20ref%29) (ShotDirection :type Vector%20%28by%20ref%29 :default "0, 0, 0") (AmmoType :type AMMO_TYPES%20Enum :default "Regular"))
  (bind (_bblockinghit _binitialoverlap _time _distance _location _impactpoint _normal _impactnormal _physmat _hitactor) (Collision|BreakHitResult Hit))
  (bind _skeletalmesh (Variables|Default|GetSkeletalMesh))
  (Utilities|FlowControl|Sequence
    (:then_0
      (switch Utilities|FlowControl|Switch|SwitchonAMMO_TYPES AmmoType
        (:Regular
          (Niagara|SpawnSystemAttached "/Game/ParticleSystems/MuzzelFlashVFX/NS_Muzzleflash_Regular_And_Rapid.NS_Muzzleflash_Regular_And_Rapid" _skeletalmesh "Muzzle" "0, 0, 0" "0.000000,-90.000000,0.000000" "SnapToTarget" false))
        (:Bouncing
          (Niagara|SpawnSystemAttached "/Game/ParticleSystems/MuzzelFlashVFX/NS_Muzzleflash_Bouncing.NS_Muzzleflash_Bouncing" _skeletalmesh "Muzzle" "0, 0, 0" "0.000000,-90.000000,0.000000" "SnapToTarget" false))
        (:Explosive
          (Niagara|SpawnSystemAttached "/Game/ParticleSystems/MuzzelFlashVFX/NS_Muzzleflash_Regular_And_Rapid.NS_Muzzleflash_Regular_And_Rapid" _skeletalmesh "Muzzle" "0, 0, 0" "0.000000,-90.000000,0.000000" "SnapToTarget" false))
        (:Flare
          (Niagara|SpawnSystemAttached "/Game/ParticleSystems/MuzzelFlashVFX/NS_Muzzleflash_flare.NS_Muzzleflash_flare" _skeletalmesh "Muzzle" "0, 0, 0" "0.000000,-90.000000,0.000000" "SnapToTarget" false))
        (:Rapid
          (Niagara|SpawnSystemAttached "/Game/ParticleSystems/MuzzelFlashVFX/NS_Muzzleflash_Regular_And_Rapid.NS_Muzzleflash_Regular_And_Rapid" _skeletalmesh "Muzzle" "0, 0, 0" "0.000000,-90.000000,0.000000" "SnapToTarget" false))
        (:Shotgun
          (Niagara|SpawnSystemAttached "/Game/ParticleSystems/MuzzelFlashVFX/NS_Muzzleflash_Shotgun.NS_Muzzleflash_Shotgun" _skeletalmesh "Muzzle" "0, 0, 0" "0.000000,-90.000000,0.000000" "SnapToTarget" false))))
    (:then_1
      ;[1 1 1] HUD No Ammo
      (if (and (Utilities|Enum|Equal(Enum) (Variables|Default|GetCurrentAmmoType) AmmoType) (<= (Variables|Default|GetCurrentMag) 0))
        (Audio|SpawnSound2D "/Game/Audio/SFX/Thesis/EmptyCue_Cue.EmptyCue_Cue" 1.0 1.0 0.0 0)
        (bind _returnvalue (UserInterface|CreateWidget "/Game/UserInterface/W_NoAmmo.W_NoAmmo_C"))
        (UserInterface|Viewport|AddtoViewport _returnvalue 0)
        (Variables|Default|SetbNoAmmo true)))
    (:then_2
      ;[1 1 1] Skjutljud + Switch Ammo
      (bind _asbp_first_person_character (Utilities|Casting|CastToBP_FirstPersonCharacter (Game|GetPlayerCharacter 0)))
      (switch Utilities|FlowControl|Switch|SwitchonAMMO_TYPES AmmoType
        (:Regular
          (Animation|Montage|PlayMontage (Variables|/Script/Acopalyps.AcopalypsCharacter|GetMesh1P _asbp_first_person_character) "/Game/Animations/CharacterAnimation/PlayerCharacter/Fire_Reg_Montage.Fire_Reg_Montage"
            (:then
              (Components|Animation|PlayAnimation (Variables|Default|GetSkeletalMesh) "/Game/Animations/CharacterAnimation/PlayerCharacter/Pistol_Fire_Anim.Pistol_Fire_Anim" false)
              (Audio|SpawnSound2D "/Game/Audio/SFX/Player/Weapon/Default/ShootDefaultLayered.ShootDefaultLayered" 1.0 1.0 0.0 0))))
        (:Bouncing
          (Animation|Montage|PlayMontage (Variables|/Script/Acopalyps.AcopalypsCharacter|GetMesh1P _asbp_first_person_character) "/Game/Animations/CharacterAnimation/PlayerCharacter/Fire_Reg_Montage.Fire_Reg_Montage"
            (:then
              (Components|Animation|PlayAnimation (Variables|Default|GetSkeletalMesh) "/Game/Animations/CharacterAnimation/PlayerCharacter/Pistol_Fire_Anim.Pistol_Fire_Anim" false)
              (Audio|SpawnSound2D "/Game/Audio/SFX/Player/Weapon/Default/ShootRicochetLayered.ShootRicochetLayered" 1.0 1.0 0.0 0))))
        (:Explosive
          (Animation|Montage|PlayMontage (Variables|/Script/Acopalyps.AcopalypsCharacter|GetMesh1P _asbp_first_person_character) "/Game/Animations/CharacterAnimation/PlayerCharacter/Fire_Launcher_Montage.Fire_Launcher_Montage"
            (:then
              (Components|Animation|PlayAnimation (Variables|Default|GetSkeletalMesh) "/Game/Animations/CharacterAnimation/PlayerCharacter/Pistol_Fire_Anim.Pistol_Fire_Anim" false)
              (Audio|SpawnSound2D "/Game/Audio/SFX/Player/Weapon/Explosive/S_RocketLaunchCue.S_RocketLaunchCue" 1.0 1.0 0.0 0))))
        (:Flare
          (Animation|Montage|PlayMontage (Variables|/Script/Acopalyps.AcopalypsCharacter|GetMesh1P _asbp_first_person_character) "/Game/Animations/CharacterAnimation/PlayerCharacter/Fire_Launcher_Montage.Fire_Launcher_Montage"
            (:then
              (Components|Animation|PlayAnimation (Variables|Default|GetSkeletalMesh) "/Game/Animations/CharacterAnimation/PlayerCharacter/Pistol_Fire_Anim.Pistol_Fire_Anim" false)
              (Audio|SpawnSound2D "/Game/Audio/SFX/Player/Weapon/Flare/S_Flare_LauncherCue.S_Flare_LauncherCue" 1.0 1.0 0.0 0))))
        (:Rapid
          (Animation|Montage|PlayMontage (Variables|/Script/Acopalyps.AcopalypsCharacter|GetMesh1P _asbp_first_person_character) "/Game/Animations/CharacterAnimation/PlayerCharacter/Fire_Rapid_Montage.Fire_Rapid_Montage"
            (:then
              (Components|Animation|PlayAnimation (Variables|Default|GetSkeletalMesh) "/Game/Animations/CharacterAnimation/PlayerCharacter/Pistol_Fire_Rapid_Anim.Pistol_Fire_Rapid_Anim" false)
              (Audio|SpawnSound2D "/Game/Audio/SFX/Player/Weapon/Default/ShootRapidLayered.ShootRapidLayered" 1.0 1.0 0.0 0))))
        (:Shotgun
          (Animation|Montage|PlayMontage (Variables|/Script/Acopalyps.AcopalypsCharacter|GetMesh1P _asbp_first_person_character) "/Game/Animations/CharacterAnimation/PlayerCharacter/Fire_Shotgun_Montage.Fire_Shotgun_Montage"
            (:then
              (Components|Animation|PlayAnimation (Variables|Default|GetSkeletalMesh) "/Game/Animations/CharacterAnimation/PlayerCharacter/Pistol_Fire_Anim.Pistol_Fire_Anim" false)
              (Audio|SpawnSound2D "/Game/Audio/SFX/Player/Weapon/Shotgun/ShotgunFireCue.ShotgunFireCue" 1.0 1.0 0.0 0))))))
    (:then_3
      ;[1 1 1] Enemy Material Hit Sound
      (bind _asbp_enemy_aicharacter (Utilities|Casting|CastToBP_EnemyAICharacter _hitactor)
        (:then
          (Audio|SpawnSoundatLocation "/Game/Audio/SFX/Combat/Enemy/Human/Flesh/BulletHitFleshCue.BulletHitFleshCue" _impactpoint "0, 0, 0" 1.0 1.0 0.0 0 0)
          (if (> (Class|EnemyAICharacter|GetHealthPercent _asbp_enemy_aicharacter) 0.0)
            (if (== (Math|Random|RandomIntegerinRange 0 4) 0) :!label _label
              (Audio|SpawnSound2D "/Game/Audio/SFX/Player/VoiceLines/S_PlayerCombatLiners.S_PlayerCombatLiners" 1.0 1.0 0.0 0))))
        (:CastFailed
          (Audio|SpawnSoundatLocation "/Game/Audio/SFX/Player/Weapon/ImpactWall/S_BulletImpactConcrete.S_BulletImpactConcrete" _impactpoint "0, 0, 0" 1.0 1.0 0.0 0 0))))
    (:then_4
      (bind _asbp_enemy_drone_base_actor (Utilities|Casting|CastToBP_EnemyDroneBaseActor _hitactor))
      (if (> (Class|EnemyDroneBaseActor|GetHealthPercent _asbp_enemy_drone_base_actor) 0.0)
        (goto _label)))))

(event EventOnCanFire
  (params (AmmoType :type AMMO_TYPES%20Enum :default "Regular"))
  (bind _skeletalmesh (Variables|Default|GetSkeletalMesh))
  ;[1 1 1] Ready Secondary Sound
  (switch Utilities|FlowControl|Switch|SwitchonAMMO_TYPES AmmoType
    (:Explosive
      (Audio|SpawnSoundAttached "/Game/Audio/SFX/Player/Weapon/Management/Rocket_ReadyCue.Rocket_ReadyCue" _skeletalmesh "None" "0, 0, 0" "0, 0, 0" "KeepRelativeOffset" false 1.0 1.0 0.0 0 0))
    (:Flare
      (Audio|SpawnSoundAttached "/Game/Audio/SFX/Player/Weapon/Management/S_SecondaryReadyCue.S_SecondaryReadyCue" _skeletalmesh "None" "0, 0, 0" "0, 0, 0" "KeepRelativeOffset" false 1.0 1.0 0.0 0 0))
    (:Shotgun
      (Audio|SpawnSoundAttached "/Game/Audio/SFX/Player/Weapon/Management/ShotgunReadyCue.ShotgunReadyCue" _skeletalmesh "None" "0, 0, 0" "0, 0, 0" "KeepRelativeOffset" false 1.0 1.0 0.0 0 0))))

(event EventTick
  (params (DeltaSeconds :type Float%20%28single-precision%29))
  (bind _flashlight (Variables|Default|GetFlashlight))
  (bind _returnvalue (Transformation|GetWorldRotation _flashlight))
  (Utilities|FlowControl|Sequence
    (:then_0
      (if (Variables|Default|GetbNoAmmo)
        (if (> (Variables|Default|GetCurrentMag) 0)
          ;[1 1 1] Event Reload Complete
          (Widget|RemovefromParent (stale EventFireTriggerEvent _returnvalue))
          (Variables|Default|SetbNoAmmo false))))
    (:then_1
      ;[1 1 1] Rotate Flashlight Towards Crosshair
      (bind (_hit _shotdirection _returnvalue_2) (Class|Gun|HitTrace))
      (if _returnvalue_2
        (Transformation|SetWorldRotation _flashlight (Math|Rotator|Lerp(Rotator) _returnvalue (Math|Rotator|FindLookatRotation (+ (Math|Vector|RotateVector "-10.000000,0.000000,8.000000" _returnvalue) (Transformation|GetWorldLocation _flashlight)) (.ImpactPoint (Collision|BreakHitResult _hit))) 0.1 true) false false)))))

(fn ConstructionScript)