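; Mission trigger volume that advances the player's mission when a BP_FirstPersonCharacter overlaps it.
; A DoOnce gate, re-armed by OnReset, passes the new mission to the character and plays the trigger clip plus a short cue sound.
; Flags optionally set RedTriggerUnlocked or mark the final trigger, which waits for the clip's duration before opening the main menu map.
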(event OnComponentBeginOverlap(Trigger)
  (params (OverlappedComponent :type Primitive%20Component%20Object%20Reference) (OtherActor :type Actor%20Object%20Reference) (OtherComp :type Primitive%20Component%20Object%20Reference) (OtherBodyIndex :type Integer) (bFromSweep :type Boolean) (SweepResult :type Hit%20Result%20Structure%20%28by%20ref%29))
  (bind _triggersoundclip (Variables|Default|GetTriggerSoundClip))
  (bind _asbp_first_person_character (Utilities|Casting|CastToBP_FirstPersonCharacter OtherActor))
  (Utilities|FlowControl|DoOnce false
    (:Completed
      (Default|UpdateMission _asbp_first_person_character (Variables|Default|GetNewMissionToSet))
      (if (Variables|Default|GetUnlockRedTrigger)
        (Variables|Default|SetRedTriggerUnlocked true))
      (Audio|PlaySound2D _triggersoundclip 1.0 1.0 0.0 0 0)
      (Audio|PlaySound2D "/Game/Audio/UX_UI/S_BinaryStream_ShortCue.S_BinaryStream_ShortCue" 1.0 1.0 0.0 0 0)
      (if (Variables|Default|GetFinalTrigger)
        (Utilities|FlowControl|Delay (Variables|/Script/Engine.SoundBase|GetDuration _triggersoundclip))
        (Game|OpenLevel(byName) "MainMenuMap")))))

(event EventBeginPlay)

(event Collision|EventActorBeginOverlap
  (params (OtherActor :type Actor%20Object%20Reference)))

(event EventTick
  (params (DeltaSeconds :type Float%20%28single-precision%29)))

(event EventOnReset
  (bind _triggersoundclip (Variables|Default|GetTriggerSoundClip))
  (Utilities|FlowControl|DoOnce false) ; enters at Reset
)

(fn ConstructionScript)